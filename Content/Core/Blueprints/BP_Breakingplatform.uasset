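; BP_Breakingplatform is a platform that shakes when hit, then breaks away.
; A hit on the Collision component plays a timeline, with play rate set by Time, that offsets the Platform's relative Y location scaled by ShakeValue.
; When the shake finishes and DelayTime passes, it hides the Platform and disables collision instead of destroying the actor, with no reset.
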(event OnComponentHit(Collision)
  (params (HitComponent :type Primitive%20Component%20Object%20Reference) (OtherActor :type Actor%20Object%20Reference) (OtherComp :type Primitive%20Component%20Object%20Reference) (NormalImpulse :type Vector :default "0, 0, 0") (Hit :type Hit%20Result%20Structure%20%28by%20ref%29))
  ;[0.15 0.15 0.15 0.5] Shake
  (bind _shake (Timeline|Timeline Play)
    (:Update
      (Transformation|SetRelativeLocation (Variables|Default|GetPlatform) (Math|Vector|MakeVector 0.0 (* _shake (Variables|Default|GetShakeValue)) 0.0) false false))
    (:Finished
      ;[0.15 0.15 0.15 0.5] Destroy
      (Utilities|FlowControl|Delay (Variables|Default|GetDelayTime))
      (Rendering|SetVisibility (Variables|Default|GetPlatform) false false)
      (Collision|SetCollisionEnabled (Variables|Default|GetCollision) "NoCollision"))))

(fn ConstructionScript)